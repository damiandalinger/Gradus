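; Actor component that runs data-table-driven NPC dialogue with branching options.
; Activation disables player movement and actions, blends the camera to the owning actor and creates the dialogue widget; deactivation reverses this.
; Talk shows the indexed row, then follows JumpTo or spawns option buttons, blocking further advancing.
; "Finish" rows flag the end and set the next conversation's start from ContinueFrom or a random eligible row.
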(event Custom|ActivateDialogue
  (bind _returnvalue (Game|GetPlayerCharacter 0))
  (if (Variables|Default|GetAllowTalk)
    (Variables|Default|GetDialogueWidget
      (:then
        _)
      (:else
        ;[1 1 1] disable everything
        (Variables|Default|SetDialogueIsActive true)
        (Pawn|Components|CharacterMovement|DisableMovement (Variables|/Script/Engine.Character|GetCharacterMovement _returnvalue))
        ;;[1 0.4621 0.3251] change to player
        (bind _asbp_nur_georg_darf_ran (Utilities|Casting|CastToBP_NurGeorgDarfRan _returnvalue))
        (Variables|/Game/ThirdPerson/Blueprints/BP_NurGeorgDarfRan.BP_NurGeorgDarfRan_C|SetallowAction _asbp_nur_georg_darf_ran false)
        ;[1 1 1] camera movement
        (Game|Player|SetViewTargetwithBlend (Game|GetPlayerController 0) (Components|GetOwner) (Variables|Default|GetBlendTime) "VTBlend_EaseInOut" 2.0 false)
        (Utilities|FlowControl|Delay (Variables|Default|GetBlendTime))
        ;[1 1 1] widget and mouse
        (bind _returnvalue_2 (UserInterface|CreateWidget "/Game/DialogueSystem/WB_Dialogue.WB_Dialogue_C"))
        (bind _output_get (Variables|Default|SetDialogueWidget _returnvalue_2))
        (UserInterface|Viewport|AddtoViewport _output_get 0)))
    ;[1 0.5534 0.3266] maybe change to interface?
    (CallFunction|Talk (Variables|Default|GetDialogueIndex))
    (else
      (Class|BPIDialogue|DeactivateDialogue(Message) (Components|GetOwner)))))

(event Custom|DeactivateDialogue
  (bind _returnvalue (Game|GetPlayerController 0))
  (Variables|Default|SetAllowTalk false)
  ;[1 1 1] remove widget
  (bind _dialoguewidget (Variables|Default|GetDialogueWidget)
    (:then
      (Widget|RemovefromParent _dialoguewidget)
      (Variables|Default|SetDialogueWidget 0)
      ;[1 1 1] camera movement back to player
      (Game|Player|SetViewTargetwithBlend (Game|GetPlayerController 0) (Game|GetPlayerCharacter 0) (Variables|Default|GetBlendTime) "VTBlend_EaseInOut" 2.0 false)
      (Utilities|FlowControl|Delay (Variables|Default|GetBlendTime))
      ;[1 1 1] enable all settings for gameplay again and hide everything for dialogue
      (Variables|/Script/Engine.PlayerController|SetbShowMouseCursor _returnvalue false)
      (Input|SetInputModeGameOnly _returnvalue false)
      (Pawn|Components|CharacterMovement|SetMovementMode (Variables|/Script/Engine.Character|GetCharacterMovement (Game|GetPlayerCharacter 0)) "MOVE_Walking" 0)
      (bind _asbp_nur_georg_darf_ran (Utilities|Casting|CastToBP_NurGeorgDarfRan (Game|GetPlayerCharacter 0)))
      (Variables|/Game/ThirdPerson/Blueprints/BP_NurGeorgDarfRan.BP_NurGeorgDarfRan_C|SetallowAction _asbp_nur_georg_darf_ran true)
      (Variables|Default|SetDialogueIsActive false)
      (Variables|Default|SetFinishDialogue false)
      (Variables|Default|SetAllowTalk true))
    (:else)))

(fn Talk
  (params (DialogueIndex :type Integer))
  (bind _returnvalue (Game|GetPlayerController 0))
  ;[1 1 1] update index, get all data from the data table row and update text of the dialogue
  (Variables|Default|SetDialogueIndex DialogueIndex)
  (bind _outrownames (DataTable|GetDataTableRowNames (Variables|Default|GetDialogue%20Table)))
  (bind _returnvalue_2 (Utilities|GetDataTableRow (Variables|Default|GetDialogue%20Table) (Utilities|Array|Get(acopy) _outrownames (Variables|Default|GetDialogueIndex)))
    (:then
      (bind _output_get (LocalVariables|SetCurrentRow _returnvalue_2))
      (Variables|/Script/UMG.TextBlock|SetText (Variables|/Game/DialogueSystem/WB_Dialogue.WB_Dialogue_C|GetTextBlock_1 (Variables|Default|GetDialogueWidget)) (.Text (Utilities|Struct|BreakS_DialogueInfo _output_get)))
      (Variables|Default|SetDialogueIndex (Math|Conversions|ToInteger(Byte) (Utilities|String|ToString(Text) (.JumpTo (Utilities|Struct|BreakS_DialogueInfo _output_get)))))
      ;[1 1 1] check if dialogue has options and if yes show them
      (if (Utilities|Array|IsNotEmpty (.Options (Utilities|Struct|BreakS_DialogueInfo _output_get)))
        (bind _array_element (Utilities|Array|ForEachLoopwithBreak (.Options (Utilities|Struct|BreakS_DialogueInfo _output_get)))
          (:LoopBody
            (bind _returnvalue_3 (UserInterface|CreateWidget "/Game/DialogueSystem/WB_DialogueOptions.WB_DialogueOptions_C" 0 (.OptionsText (Utilities|Struct|BreakS_OptionsInfo _array_element)) (.JumpTo (Utilities|Struct|BreakS_OptionsInfo _array_element)) self))
            (Widget|Panel|AddChild (Variables|/Game/DialogueSystem/WB_Dialogue.WB_Dialogue_C|GetOptionsBox (Variables|Default|GetDialogueWidget)) _returnvalue_3)
            ;[1 1 1] enable mouse input for option selecting
            (Variables|/Script/Engine.PlayerController|SetbShowMouseCursor _returnvalue true)
            (Input|SetInputModeGameandUI _returnvalue 0 "DoNotLock" false true)
            ;[1 1 1] disable so player cant spam input
            (Variables|Default|SetAllowTalk false)))
        (else
          ;[1 1 1] if no options, check if this line is the last one and set finish for next activation of the dialogue
          (Widget|Panel|ClearChildren (Variables|/Game/DialogueSystem/WB_Dialogue.WB_Dialogue_C|GetOptionsBox (Variables|Default|GetDialogueWidget)))
          (if (Utilities|Enum|Equal(Enum) (.JumpTo (Utilities|Struct|BreakS_DialogueInfo (LocalVariables|GetCurrentRow))) (Utilities|Text|MakeLiteralText "Finish"))
            (Variables|Default|SetFinishDialogue true)
            ;[1 1 1] select a random available dialogue and set the dialogue index to its row name
            (if (Utilities|Enum|Equal(Enum) (Utilities|String|ToString(Text) (.ContinueFrom (Utilities|Struct|BreakS_DialogueInfo (LocalVariables|GetCurrentRow)))) "Random")
              (Utilities|Array|Clear (LocalVariables|GetRandomDialogues))
              (bind _outrownames_2 (DataTable|GetDataTableRowNames (Variables|Default|GetDialogue%20Table)))
              (for _array_element_2 _outrownames_2
                (bind _returnvalue_4 (Utilities|GetDataTableRow (Variables|Default|GetDialogue%20Table) _array_element_2)
                  (:then
                    (if (.Random (Utilities|Struct|BreakS_DialogueInfo _returnvalue_4))
                      (Utilities|Array|Add (LocalVariables|GetRandomDialogues) _array_element_2)))))
              (Variables|Default|SetDialogueIndex (Math|Conversions|ToInteger(Byte) (Utilities|String|ToString(Name) (.OutItem (Utilities|Array|Random (LocalVariables|GetRandomDialogues))))))
              (else
                (Variables|Default|SetDialogueIndex (Math|Conversions|ToInteger(Byte) (Utilities|String|ToString(Text) (.ContinueFrom (Utilities|Struct|BreakS_DialogueInfo (LocalVariables|GetCurrentRow))))))))))))))