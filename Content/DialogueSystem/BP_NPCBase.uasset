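; Base NPC actor that gives a character an interact prompt and dialogue with the player.
; A Box overlap with the player shows or hides InteractText, which rotates toward the camera on Tick while in range.
; Activate, Deactivate and Talk events forward to BPCDialogueSystem, toggling the prompt and closing dialogue when Talk follows a finish line.
; Deactivation also prints a leftover-style "Hello" debug string.
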(event OnComponentBeginOverlap(Box)
  (params (OverlappedComponent :type Primitive%20Component%20Object%20Reference) (OtherActor :type Actor%20Object%20Reference) (OtherComp :type Primitive%20Component%20Object%20Reference) (OtherBodyIndex :type Integer) (bFromSweep :type Boolean) (SweepResult :type Hit%20Result%20Structure%20%28by%20ref%29))
  ;[1 1 1] show and hide interact text
  (if (== OtherActor (Game|GetPlayerCharacter 0))
    (Development|SetHiddeninGame (Variables|Default|GetInteractText) false false)
    (Variables|Default|SetRotateText true)))

(event OnComponentEndOverlap(Box)
  (params (OverlappedComponent :type Primitive%20Component%20Object%20Reference) (OtherActor :type Actor%20Object%20Reference) (OtherComp :type Primitive%20Component%20Object%20Reference) (OtherBodyIndex :type Integer))
  ;[1 1 1] show and hide interact text
  (if (== OtherActor (Game|GetPlayerCharacter 0))
    (Development|SetHiddeninGame (Variables|Default|GetInteractText) true false)
    (Variables|Default|SetRotateText false)))

(event EventTick
  (params (DeltaSeconds :type Float%20%28single-precision%29))
  (bind _interacttext (Variables|Default|GetInteractText))
  ;[1 1 1] interact text always rotate towards camera
  (if (Variables|Default|GetRotateText)
    (Transformation|SetWorldRotation _interacttext (Math|Rotator|FindLookatRotation (Transformation|GetWorldLocation _interacttext) (Transformation|GetWorldLocation (Variables|/Script/Engine.Actor|GetRootComponent (Game|GetPlayerCameraManager 0)))) false false)))

(event EventDeactivateDialogue
  (bind _bpc_dialoguesystem (Variables|Default|GetBPC_DialogueSystem))
  (if (Variables|/Game/DialogueSystem/BPC_DialogueSystem.BPC_DialogueSystem_C|GetDialogueIsActive _bpc_dialoguesystem)
    (Default|DeactivateDialogue _bpc_dialoguesystem)
    (Development|SetHiddeninGame (Variables|Default|GetInteractText) false false)
    (Development|PrintString "Hello")))

(event EventTalk
  (params (DialogueIndex :type Integer))
  ;[1 1 1] if last dialogue line was a finish line, deactivate the dialogue
  (if (not (Variables|/Game/DialogueSystem/BPC_DialogueSystem.BPC_DialogueSystem_C|GetFinishDialogue (Variables|Default|GetBPC_DialogueSystem)))
    (Default|Talk (Variables|Default|GetBPC_DialogueSystem) DialogueIndex)
    (else
      (CallFunction|DeactivateDialogue))))

(event EventActivateDialogue
  (Default|ActivateDialogue (Variables|Default|GetBPC_DialogueSystem))
  (Development|SetHiddeninGame (Variables|Default|GetInteractText) true false))

(fn ConstructionScript)