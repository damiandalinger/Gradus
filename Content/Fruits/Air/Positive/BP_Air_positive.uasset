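; Gameplay ability for the positive Air fruit: a short forward dash that damages pawns along the way.
; Activation disables input, plays a montage, applies constant-force root motion and sets the owning mesh to ignore Pawn and Visibility channels.
; A looping timer box-overlaps around the avatar, sending damage and stun once per actor via a tracking list.
; The dash's finish re-enables input and ends the ability, without restoring collision or explicitly clearing the timer.
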(event Custom|CustomEvent
  (bind _returnvalue (Ability|GetAvatarActorfromActorInfo))
  (bind (_outactors _returnvalue_2) (Collision|BoxOverlapActors (Transformation|GetActorLocation _returnvalue) "100.000000,100.000000,100.000000" (Utilities|Array|MakeArray "ObjectTypeQuery3") 0 (Utilities|Array|MakeArray _returnvalue) :!class /Script/Engine.KismetSystemLibrary))
  (for _array_element _outactors
    (if _returnvalue_2
      (if (not (Utilities|Array|ContainsItem (Variables|Default|GetTakeDamage) _array_element))
        (Utilities|Array|Add (Variables|Default|GetTakeDamage) _array_element)
        (Class|BPIDamagable|TakeDamage(Message) _array_element (Utilities|Struct|MakeS_DamageInfo 2e+01 2e+01))))))

(event Ability|EventActivateAbility
  (bind _returnvalue (Class|GameplayAbility|GetOwningComponentfromActorInfo))
  (bind _returnvalue_2 (Ability|GetAvatarActorfromActorInfo))
  (Ability|CommitAbility)
  (Input|DisableInput (Ability|GetAvatarActorfromActorInfo) (Game|GetPlayerController (Game|GetPlayerState 0)))
  (|PlayMontageandWaitProxy "None" (Variables|Default|GetMontage%20to%20Play) 1.0 "None" true 1.0 0.0 false
    (:then
      (Ability|Tasks|ApplyRootMotionConstantForce "None" (Transformation|GetActorForwardVector _returnvalue_2) 3e+03 0.2 false 0 "SetVelocity" (Transformation|GetVelocity _returnvalue_2)
        (:then
          (Collision|SetCollisionResponsetoChannel _returnvalue "ECC_Visibility" "ECR_Ignore")
          (Collision|SetCollisionResponsetoChannel _returnvalue "ECC_Pawn" "ECR_Ignore")
          (Utilities|Time|SetTimerbyEvent (delegate Custom|CustomEvent) 0.05 true))
        (:OnFinish
          (Ability|EndAbility)
          (Input|EnableInput (Ability|GetAvatarActorfromActorInfo) (Game|GetPlayerController (Game|GetPlayerState 0))))))))

(event Ability|EventOnEndAbility
  (params (bWasCancelled :type Boolean))
  (Development|PrintString "Air positive"))

(fn NewFunction)