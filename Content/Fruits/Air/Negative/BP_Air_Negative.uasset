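; Air_Negative is a Gameplay Ability that plays the AirNegative montage and spawns a Niagara effect at the avatar.
; Activation commits the ability, starts the montage, then spawns the effect and ends the ability without waiting for the montage to finish.
; A custom event with DeltaSeconds moves the effect to the avatar's location, but nothing here calls it.
; Debug prints and an empty Tick graph suggest a work-in-progress prototype.
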(event Custom|CustomEvent_1
  (params (DeltaSeconds :type Float%20%28single-precision%29))
  (Development|PrintString "Suck Egg")
  (Transformation|SetWorldLocation (stale Ability|EventActivateAbility _returnvalue_3) (.location (Transformation|GetActorTransform (Ability|GetAvatarActorfromActorInfo))) true false))

(event Ability|EventActivateAbility
  (bind _returnvalue (Ability|GetAvatarActorfromActorInfo))
  (bind _returnvalue_2 (Transformation|GetActorTransform _returnvalue))
  (Development|PrintString "Hello")
  (Ability|CommitAbility)
  (|PlayMontageandWaitProxy "None" (Variables|Default|GetAir_Negative) 1.0 "None" true 1.0 0.0 false
    (:then
      (bind _returnvalue_3 (Niagara|SpawnSystematLocation "/Game/NiagaraKurs/NiagaraBasic/11-UVTest/NS_UVTesto.NS_UVTesto" (.location _returnvalue_2) (.rotation _returnvalue_2) (.scale _returnvalue_2)))
      (Ability|EndAbility))))

(event Ability|EventOnEndAbility
  (params (bWasCancelled :type Boolean))
  (Development|PrintString "Air_Negative"))

(event Custom|CustomEvent
  (params (DeltaSeconds :type Float%20%28single-precision%29)))