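; BP_PatrolRoute is an enemy AI patrol route defined by the points of a Spline component.
; GetSplinePointAsWorldPosition returns the world location of the point at CurrentPointIndex.
; IncrementPatrolRoute steps that index by Direction, flipping Direction at the last and first points so the route runs back and forth rather than looping.
; The index and direction are stored on the route itself.
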(event Custom|Increment%20Patrol%20Route
  (bind _output_get (Variables|Default|SetcurrentPointIndex (+ (Variables|Default|GetcurrentPointIndex) (Variables|Default|GetDirection))))
  (if (== _output_get (- (Spline|GetNumberOfSplinePoints (Variables|Default|GetSpline)) 1))
    (Variables|Default|SetDirection -1)
    (elif (== (Variables|Default|GetcurrentPointIndex) 0)
      (Variables|Default|SetDirection 1))))

(fn ConstructionScript)

(fn GetSplinePointasWorldPosition
  (return (Spline|GetLocationatSplinePoint (Variables|Default|GetSpline) (Variables|Default|GetcurrentPointIndex) "World")))