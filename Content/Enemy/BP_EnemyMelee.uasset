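; Melee enemy Blueprint that handles a sword attack and its own death sequence.
; Attack plays a slash montage whose notify runs a forward pawn sphere trace to deal damage, signalling attack end on completion or interruption.
; Death hides UI, clears the player's lock-on and stops the AI.
; After a delay it relocates an existing BP_Glühwürmchen beside itself and sets it attacking the player, working around broken spawning; the actor is never destroyed.
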(event EventBeginPlay
  (|CallParentFunction) ; This node is disabled and will not be called.\nDrag off pins to build functionality.
)

(event Collision|EventActorBeginOverlap
  (params (OtherActor :type Actor%20Object%20Reference)))

(event EventTick
  (params (DeltaSeconds :type Float%20%28single-precision%29)))

(event EventAttack
  (bind _returnvalue (Transformation|GetActorLocation))
  (bind _notifyname (Animation|Montage|PlayMontage (Variables|Character|GetMesh) "/Game/Animations/Stable_Sword_Outward_Slash__1__Anim_mixamo_com_Montage1.Stable_Sword_Outward_Slash__1__Anim_mixamo_com_Montage1")
    (:OnCompleted
      (Default|CallOnAttackEnd :!label _label))
    (:OnInterrupted
      (goto _label))
    (:OnNotifyBegin
      (switch name _notifyname
        (:Slash
          (bind (_outhit _returnvalue_2) (Collision|SphereTraceForObjects _returnvalue (+ _returnvalue (* (Transformation|GetActorForwardVector) 2e+02)) 2e+01 (Utilities|Array|MakeArray "ObjectTypeQuery3") false 0 "ForDuration" true "(R=1.000000,G=0.000000,B=0.000000,A=1.000000)" "(R=0.000000,G=1.000000,B=0.000000,A=1.000000)" 2.0))
          (if _returnvalue_2
            (Class|BPIDamagable|TakeDamage(Message) (.HitActor (Collision|BreakHitResult _outhit)) (Utilities|Struct|MakeS_DamageInfo 3e+01 0.0 "NewEnumerator1" "NewEnumerator2"))))))))

(event EventDeath
  (bind _returnvalue (Transformation|GetActorLocation))
  (bind _aicenemybase (Variables|Default|GetAICEnemyBase))
  (Rendering|SetVisibility (Variables|Default|GetStunMeter) false false)
  (Rendering|SetVisibility (Variables|Default|GetHealthBar) false false)
  (Rendering|SetVisibility (Variables|Default|GetLockImage) false false)
  (bind _asbp_georg (Utilities|Casting|CastToBP_Georg (Game|GetPlayerCharacter 0)))
  (Variables|/Game/ThirdPerson/Blueprints/BP_Georg.BP_Georg_C|SetLockedOnTarget _asbp_georg 0)
  (Default|SetStateasDead _aicenemybase)
  (AI|Logic|StopLogic (Variables|/Script/AIModule.AIController|GetBrainComponent _aicenemybase) "Alkoholvergiftung")
  (Utilities|FlowControl|Delay 2.0)
  ;[1 1 1] becauseactor spawning does not work atm
  (bind _returnvalue_2 (Actor|GetActorOfClass "/Game/Enemy/BP_Glühwürmchen.BP_Glühwürmchen_C"))
  (Transformation|SetActorLocation _returnvalue_2 (+ _returnvalue "50.000000,0.000000,0.000000") false false)
  (bind _asaic_enemy_base (Utilities|Casting|CastToAIC_EnemyBase (AI|GetAIController _returnvalue_2)))
  (Default|SetStateasAttack _asaic_enemy_base (Game|GetPlayerCharacter 0))
  (AI|Components|Blackboard|SetValueasVector (Variables|/Script/AIModule.AIController|GetBlackboard (AI|GetAIController _returnvalue_2)) (Utilities|Name|MakeLiteralName "PointOfInterest") _returnvalue)
  (AI|Components|Blackboard|SetValueasObject (Variables|/Script/AIModule.AIController|GetBlackboard (AI|GetAIController _returnvalue_2)) (Utilities|Name|MakeLiteralName "SelfActor") self))

(fn ConstructionScript
  (|CallParentFunction))