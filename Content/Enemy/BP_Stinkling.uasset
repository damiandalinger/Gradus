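; BP_Stinkling is an enemy Blueprint that defines a melee-range Attack event.
; Attack runs a short forward sphere trace against Pawns with timed debug drawing, but nothing consumes the hit result.
; It then plays the AM_Cast montage on the mesh and fires the OnAttackEnd dispatcher on completion or interruption.
; BeginPlay, Tick, overlap and construction add no logic of their own.
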(event EventBeginPlay
  (|CallParentFunction) ; This node is disabled and will not be called.\nDrag off pins to build functionality.
)

(event Collision|EventActorBeginOverlap
  (params (OtherActor :type Actor%20Object%20Reference)))

(event EventTick
  (params (DeltaSeconds :type Float%20%28single-precision%29)))

(event EventAttack
  (bind _returnvalue (Transformation|GetActorLocation))
  (Collision|SphereTraceForObjects _returnvalue (+ _returnvalue (* (Transformation|GetActorForwardVector) 2e+02)) 2e+01 (Utilities|Array|MakeArray "ObjectTypeQuery3") false 0 "ForDuration" true "(R=1.000000,G=0.000000,B=0.000000,A=1.000000)" "(R=0.000000,G=1.000000,B=0.000000,A=1.000000)" 1.0)
  (Animation|Montage|PlayMontage (Variables|Character|GetMesh) "/Game/Sword_Animations/Animations/Sequence1/02_Attack/01_Combo_Attack_01/AM_Cast.AM_Cast"
    (:OnCompleted
      _)
    (:OnInterrupted
      _))
  (Default|CallOnAttackEnd))

(fn ConstructionScript
  (|CallParentFunction))