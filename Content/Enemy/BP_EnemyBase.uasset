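; Base enemy Blueprint that exposes health, healing and damage functions, with health state held in a BPCDamageSystem component.
; The health getters read current and max health straight from that component.
; Heal and TakeDamage are thin pass-throughs to same-named calls, returning their results with no enemy-specific logic.
; The construction script is empty.
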(fn ConstructionScript)

(fn GetCurrentHealth
  (return (Variables|/Game/DamageSystem/BPC_DamageSystem.BPC_DamageSystem_C|GetCurrentHealth (Variables|Default|GetBPC_DamageSystem))))

(fn GetMaxHealth
  (return (Variables|/Game/DamageSystem/BPC_DamageSystem.BPC_DamageSystem_C|GetMaxHealth (Variables|Default|GetBPC_DamageSystem))))

(fn Heal
  (params (HealAmount :type Float%20%28double-precision%29))
  (bind _newhealth (CallFunction|Heal HealAmount))
  (return _newhealth))

(fn TakeDamage
  (params (DamageInfo :type S%20Damage%20Info%20Structure))
  (bind _wasdamaged (CallFunction|TakeDamage DamageInfo))
  (return _wasdamaged))