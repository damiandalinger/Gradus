(event Input|KeyboardEvents|I
  (params (Key :type Key%20Structure :default "None"))
  (bind _returnvalue (Game|GetPlayerController 0))
  (:Pressed
    (Utilities|FlowControl|FlipFlop
      (:A
        (Variables|Default|GetInventory%20Widget
          (:then
            (Widget|SetVisibility (Variables|Default|GetInventory%20Widget) "Visible"))
          (:else
            (bind _returnvalue_2 (UserInterface|CreateWidget "/Game/Inventory/WB_Inventory.WB_Inventory_C" (Game|GetPlayerController 0)))
            (bind _output_get (Variables|Default|SetInventory%20Widget _returnvalue_2))
            (UserInterface|Viewport|AddtoViewport _output_get 0)))
        (Input|SetInputModeGameandUI _returnvalue 0 "DoNotLock" true false)
        (Variables|/Script/Engine.PlayerController|SetbShowMouseCursor (Game|GetPlayerController 0) true)
        (Game|SetGamePaused true))
      (:B
        (bind _inventory_widget (Variables|Default|GetInventory%20Widget)
          (:then
            (Widget|SetVisibility _inventory_widget "Hidden")
            (Input|SetInputModeGameOnly _returnvalue false)
            (Variables|/Script/Engine.PlayerController|SetbShowMouseCursor _returnvalue false)
            (Game|SetGamePaused false))
          (:else))))))

(event Input|KeyboardEvents|E
  (params (Key :type Key%20Structure :default "None"))
  (:Pressed
    (Variables|Default|GetInventory%20Widget
      (:then
        _)
      (:else
        (bind _returnvalue (UserInterface|CreateWidget "/Game/Inventory/WB_Inventory.WB_Inventory_C"))
        (bind _output_get (Variables|Default|SetInventory%20Widget _returnvalue))
        (UserInterface|Viewport|AddtoViewport _output_get 0)
        (Widget|SetVisibility (Variables|Default|GetInventory%20Widget) "Hidden")))
    (for _array_element (Collision|GetOverlappingActors "/Game/Inventory/BP_Item.BP_Item_C" :!class /Script/Engine.Actor)
      (if (Utilities|DoesObjectImplementInterface _array_element "/Game/Inventory/BPI_Pickup.BPI_Pickup_C")
        (bind _item (Class|BPIPickup|PickUpItem(Message) _array_element))
        (Default|AddItemtoInventory (Variables|Default|GetBPC_Inventory) _item)))))

(fn ConstructionScript)