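; BPC_DamageSystem is a damage component that tracks an owner's health and death state.
; Heal adds health clamped to the maximum while alive.
; TakeDamage takes a DamageInfo struct, gated by CanBeDamaged's exec outputs for death and invincibility, which the hit can override.
; Lethal hits set IsDead and call OnDeath; survivable hits call OnDamageRespone with the response type only when interruptible or forced.
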(event EventBeginPlay)

(event EventTick
  (params (DeltaSeconds :type Float%20%28single-precision%29)))

(fn Heal
  (params (HealAmount :type Float%20%28double-precision%29))
  (if (not (Variables|Default|GetisDead))
    (bind _output_get (Variables|Default|SetCurrentHealth (Math|Float|Clamp(Float) (+ HealAmount (Variables|Default|GetCurrentHealth)) 0.0 (Variables|Default|GetMaxHealth))))
    (return _output_get)))

(fn TakeDamage
  (params (DamageInfo :type S%20Damage%20Info%20Structure))
  (bind (_damage _knockbackamount _damagetype _damageresponse _shoulddamageinvincible _shouldforceinterrupt) (Utilities|Struct|BreakS_DamageInfo DamageInfo))
  (Utilities|CanbeDamaged _shoulddamageinvincible
    (:DoDamage
      (bind _output_get (Variables|Default|SetCurrentHealth (- (Variables|Default|GetCurrentHealth) _damage)))
      (if (<= _output_get 0.0)
        (Variables|Default|SetisDead true)
        (Default|CallOnDeath)
        (return true)
        (elif (or (Variables|Default|GetisInterruptible) _shouldforceinterrupt)
          (Default|CallOnDamageRespone _damageresponse)
          (return true))))
    (:NoDamage
      (return false))))