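; Metal bolt projectile actor that damages the actor it hits.
; On BeginPlay it binds the mesh's component hit event, which passes the hit actor to HandleOnHit.
; That function deactivates projectile movement, sends Damage with a fixed damage type through a TakeDamage message, and sets a short lifespan so the bolt is destroyed later.
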(event Custom|OnBoltHit
  (params (HitComponent :type Primitive%20Component%20Object%20Reference) (OtherActor :type Actor%20Object%20Reference) (OtherComp :type Primitive%20Component%20Object%20Reference) (NormalImpulse :type Vector) (Hit :type Hit%20Result%20Structure%20%28by%20ref%29))
  (CallFunction|HandleonHit OtherActor))

(event EventBeginPlay
  (Collision|BindEventtoOnComponentHit (Variables|Default|GetMetalBoltMesh) (delegate Custom|OnBoltHit)))

(fn ConstructionScript)

(fn HandleonHit
  (params (Other%20Actor :type Actor%20Object%20Reference))
  (Components|Activation|Deactivate (Variables|Default|GetProjectileMovement))
  (Class|BPIDamagable|TakeDamage(Message) Other%20Actor (Utilities|Struct|MakeS_DamageInfo (Variables|Default|GetDamage) 0.0 "NewEnumerator3" "NewEnumerator0" false false))
  (Actor|SetLifeSpan 1e+01))