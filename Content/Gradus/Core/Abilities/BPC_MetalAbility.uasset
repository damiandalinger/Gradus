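; Player ability component for a metal power that, on the shoot input, works as bolts or a chain depending on IsFruitPositive.
; When false, the first trigger spawns bolts on mesh sockets; later triggers detach a random one and launch it at the camera trace target.
; When true, it spawns one socket-attached chain facing that target, if nothing has spawned yet.
; HasSpawned is shared and never reset here; spline-stretching code is unconnected.
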(event Input|EnhancedActionEvents|EnhancedInputActionIA_Shoot
  (params (ActionValue :type Boolean) (ElapsedSeconds :type Float%20%28double-precision%29) (TriggeredSeconds :type Float%20%28double-precision%29) (InputAction :type Input%20Action%20Object%20Reference :default "/Game/ThirdPerson/Input/Actions/IA_Shoot.IA_Shoot"))
  (bind _returnvalue (CallFunction|GetTraceEnd))
  (bind _chainsocketname (Variables|ChainSettings|GetChainSocketName))
  (bind _charactermeshreference (Variables|References|GetCharacterMeshReference))
  (bind _returnvalue_2 (Transformation|GetSocketLocation _charactermeshreference _chainsocketname))
  (:Triggered
    (if (not (Variables|Config|GetIsFruitPositive))
      (if (Variables|Config|GetHasSpawned)
        ;[1 1 1] Shoot Bolt
        (CallFunction|GetRandomBolt)
        (Transformation|DetachFromActor (Variables|References|GetMetalBoltReference) "KeepWorld" "KeepWorld" "KeepWorld")
        (bind _returnvalue_3 (CallFunction|GetBoltRotation))
        (CallFunction|SetDirectionandFire _returnvalue_3)
        (else
          ;[1 1 1] Spawn Bolts
          (for _array_element (Variables|BoltSettings|GetBoltSocketNames)
            (CallFunction|SpawnBolt _array_element))
          (Variables|Config|SetHasSpawned true)
          (Variables|Config|SetTraceDistance (Variables|BoltSettings|GetBoltRange))))))
  (:Started
    (if (Variables|Config|GetIsFruitPositive)
      (if (not (Variables|Config|GetHasSpawned))
        (Variables|Config|SetHasSpawned true)
        (Variables|Config|SetTraceDistance (Variables|ChainSettings|GetChainRange))
        (bind _outhit (Collision|LineTraceByChannel (Transformation|GetWorldLocation (Variables|References|GetCameraReference)) _returnvalue "TraceTypeQuery1" false 0 "None"))
        (bind _output_get (Variables|Default|SetStartLocation _returnvalue_2))
        (bind _output_get_2 (Variables|Default|SetEndLocation (Math|Vector|SelectVector (.ImpactPoint (Collision|BreakHitResult _outhit)) _returnvalue (.bBlockingHit (Collision|BreakHitResult _outhit)))))
        (Development|PrintString (Utilities|String|Append (Utilities|String|ToString(Vector) _output_get_2) (Utilities|String|ToString(Vector) _output_get)) true true "(R=0.000000,G=0.660000,B=1.000000,A=1.000000)" 1e+02)
        (bind _returnvalue_4 (Game|SpawnActorfromClass "/Game/Gradus/Core/Abilities/BP_Chain.BP_Chain_C" (Math|Transform|MakeTransform _returnvalue_2 (Math|Rotator|FindLookatRotation _returnvalue_2 (Math|Vector|SelectVector (.ImpactPoint (Collision|BreakHitResult _outhit)) _returnvalue (.bBlockingHit (Collision|BreakHitResult _outhit))))) "Undefined" "MultiplyWithRoot" 0 0))
        (bind _output_get_3 (Variables|Default|SetChainReference _returnvalue_4))
        (Transformation|AttachComponentToComponent (Variables|/Script/Engine.Actor|GetRootComponent _output_get_3) (Variables|References|GetCharacterMeshReference) "None" "KeepWorld" "KeepWorld" "KeepWorld" true)))))

(event EventBeginPlay
  ;[1 1 1] Get References
  (CallFunction|GetPlayerReferences))

(fn GetPlayerReferences
  (bind _asbp_character_test (Utilities|Casting|CastToBP_CharacterTest (Components|GetOwner)))
  (Variables|References|SetCameraReference (Variables|/Game/Gradus/Core/Abilities/BP_CharacterTest.BP_CharacterTest_C|GetFollowCamera _asbp_character_test))
  (Variables|References|SetCharacterMeshReference (Variables|/Script/Engine.Character|GetMesh _asbp_character_test))
  (return))

(fn GetTraceEnd
  (bind _camerareference (Variables|References|GetCameraReference))
  (return (+ (Transformation|GetWorldLocation _camerareference) (* (Math|Vector|GetForwardVector _camerareference) (Variables|Config|GetTraceDistance)))))

(fn GetBoltRotation
  (bind _output_get (LocalVariables|SetTraceEnd (CallFunction|GetTraceEnd)))
  (bind _outhit (Collision|LineTraceByChannel (Transformation|GetWorldLocation (Variables|References|GetCameraReference)) _output_get "TraceTypeQuery1" false 0 "None"))
  (return (Math|Rotator|FindLookatRotation (Transformation|GetActorLocation (Variables|References|GetMetalBoltReference)) (Math|Vector|SelectVector (.ImpactPoint (Collision|BreakHitResult _outhit)) (LocalVariables|GetTraceEnd) (.bBlockingHit (Collision|BreakHitResult _outhit))))))

(fn GetRandomBolt
  (bind _asbp_metal_bolt (Utilities|Casting|CastToBP_MetalBolt (.OutItem (Utilities|Array|Random (Variables|BoltSettings|GetMetalBolts)))))
  (bind _output_get (Variables|References|SetMetalBoltReference _asbp_metal_bolt))
  (Utilities|Array|RemoveItem (Variables|BoltSettings|GetMetalBolts) _output_get)
  (return))

(fn SetDirectionandFire
  (params (NewRotation :type Rotator))
  (bind _metalboltreference (Variables|References|GetMetalBoltReference))
  (bind _returnvalue (Actor|GetComponentbyClass _metalboltreference "/Script/Engine.ProjectileMovementComponent"))
  (Transformation|SetActorRotation (Variables|References|GetMetalBoltReference) NewRotation)
  (Game|Components|ProjectileMovement|SetVelocityinLocalSpace _returnvalue (Math|Vector|MakeVector (Variables|BoltSettings|GetBoltSpeed) 0.0 0.0))
  (Components|Activation|Activate _returnvalue false)
  (Actor|SetLifeSpan (Variables|References|GetMetalBoltReference) 5.0)
  (return))

(fn SpawnBolt
  (params (InSocketName :type Name))
  (bind _returnvalue (Game|SpawnActorfromClass "/Game/Gradus/Core/Abilities/BP_MetalBolt.BP_MetalBolt_C" (Transformation|GetSocketTransform (Variables|References|GetCharacterMeshReference) InSocketName "RTS_World") "Undefined" "MultiplyWithRoot" 0 0))
  (Utilities|Array|Add (Variables|BoltSettings|GetMetalBolts) _returnvalue)
  (Transformation|AttachComponentToComponent (Variables|/Script/Engine.Actor|GetRootComponent _returnvalue) (Variables|References|GetCharacterMeshReference) "None" "KeepWorld" "KeepWorld" "KeepWorld" true)
  (return))