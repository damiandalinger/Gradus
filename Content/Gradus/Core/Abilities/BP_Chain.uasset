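; BP_Chain is an actor that builds a chain between the start and end points of the player's metal ability.
; On BeginPlay it reads both locations from BPC_MetalAbility on BP_CharacterTest and derives a segment count from their distance and the mesh length.
; It then lays interpolated spline points along that straight line, adding a spline mesh between successive points.
; The chain is built once, with no later updates.
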(event EventBeginPlay
  (bind _spline (Variables|Default|GetSpline))
  (Utilities|FlowControl|Sequence
    (:then_0
      (bind _asbp_character_test (Utilities|Casting|CastToBP_CharacterTest (Game|GetPlayerCharacter 0)))
      (Variables|Default|SetEndLocation (Variables|/Game/Gradus/Core/Abilities/BPC_MetalAbility.BPC_MetalAbility_C|GetEndLocation (Actor|GetComponentbyClass _asbp_character_test "/Game/Gradus/Core/Abilities/BPC_MetalAbility.BPC_MetalAbility_C")))
      (Variables|Default|SetStartLocation (Variables|/Game/Gradus/Core/Abilities/BPC_MetalAbility.BPC_MetalAbility_C|GetStartLocation (Actor|GetComponentbyClass _asbp_character_test "/Game/Gradus/Core/Abilities/BPC_MetalAbility.BPC_MetalAbility_C"))))
    (:then_1
      (Spline|ClearSplinePoints (Variables|Default|GetSpline) true))
    (:then_2
      (bind _output_get (Variables|Default|SetDistance (Math|Vector|VectorLength (- (Variables|Default|GetEndLocation) (Variables|Default|GetStartLocation)))))
      (bind _output_get_2 (Variables|Default|SetChainSegment (Math|Float|Ceil (/ _output_get (Variables|Default|GetMeshLength)))))
      (bind _result (Math|Integer|DecrementInt _output_get_2)
        (:%20%20
          (for _index (range 0 _result)
            (Spline|AddSplinePoint (Variables|Default|GetSpline) (Math|Vector|Lerp(Vector) (Variables|Default|GetStartLocation) (Variables|Default|GetEndLocation) (/ (Math|Conversions|ToFloat(Integer) _index) (Math|Conversions|ToFloat(Integer) (Variables|Default|GetChainSegment)))) "World" true)
            (bind _returnvalue (AddComponent|AddSplineMeshComponent false))
            (SplineMesh|SetForwardAxis _returnvalue "X" true)
            (SplineMesh|SetStartandEnd _returnvalue (.Location (Spline|GetLocationandTangentatSplinePoint _spline (- _index 1) "Local")) (.Tangent (Spline|GetLocationandTangentatSplinePoint _spline (- _index 1) "Local")) (.Location (Spline|GetLocationandTangentatSplinePoint _spline _index "Local")) (.Tangent (Spline|GetLocationandTangentatSplinePoint _spline _index "Local")) true :!class /Script/Engine.SplineMeshComponent)))))))

(fn ConstructionScript)